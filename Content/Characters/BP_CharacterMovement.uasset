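; BP_CharacterMovement is a Character Blueprint that handles player input for side-to-side movement, jumping and sliding.
; BeginPlay adds the IMC_PlayerMovement Enhanced Input mapping context to player 0's subsystem.
; Move input feeds movement along the actor's right vector only, with no forward axis, while jump starts and stops on press and release.
; Slide currently maps to plain Crouch and UnCrouch, with no extra sliding logic.
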(event Input|EnhancedActionEvents|EnhancedInputActionIA_PlayerMovementSlide
  (params (ActionValue :type Boolean) (ElapsedSeconds :type Float%20%28double-precision%29) (TriggeredSeconds :type Float%20%28double-precision%29) (InputAction :type Input%20Action%20Object%20Reference :default "/Game/Input/PlayerMovementActions/IA_PlayerMovementSlide.IA_PlayerMovementSlide"))
  ;[0.15 0.15 0.15 0.5] Slide?
  (:Started
    (Character|Crouch))
  (:Completed
    (Character|UnCrouch)))

(event Input|EnhancedActionEvents|EnhancedInputActionIA_PlayerMovemetJump
  (params (ActionValue :type Boolean) (ElapsedSeconds :type Float%20%28double-precision%29) (TriggeredSeconds :type Float%20%28double-precision%29) (InputAction :type Input%20Action%20Object%20Reference :default "/Game/Input/PlayerMovementActions/IA_PlayerMovemetJump.IA_PlayerMovemetJump"))
  ;[0.15 0.15 0.15 0.5] Jumping
  (:Started
    (Character|Jump))
  (:Completed
    (Character|StopJumping)))

(event Input|EnhancedActionEvents|EnhancedInputActionIA_PlayerMovementMove
  (params (ActionValue :type Float%20%28double-precision%29) (ElapsedSeconds :type Float%20%28double-precision%29) (TriggeredSeconds :type Float%20%28double-precision%29) (InputAction :type Input%20Action%20Object%20Reference :default "/Game/Input/PlayerMovementActions/IA_PlayerMovementMove.IA_PlayerMovementMove"))
  ;[0.15 0.15 0.15 0.5] Left and Right Movement
  (:Triggered
    (Pawn|Input|AddMovementInput (Transformation|GetActorRightVector) ActionValue false)))

(event EventBeginPlay
  ;[0.15 0.15 0.15 0.5] Setup Mapping
  (Input|AddMappingContext (PlayerController|LocalPlayerSubsystems|GetEnhancedInputLocalPlayerSubsystem (Game|GetPlayerController 0)) "/Game/Input/IMC_PlayerMovement.IMC_PlayerMovement" 0 "(bIgnoreAllPressedKeysUntilRelease=True,bForceImmediately=False,bNotifyUserSettings=False)"))

(fn ConstructionScript)