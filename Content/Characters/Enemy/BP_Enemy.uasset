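; Enemy actor whose patrol, stare and quick-time-event attack behavior runs through StateTree tasks, with older in-Blueprint logic left disconnected.
; Vision and attack-range overlaps with the player character set the flags that serve as StateTree transition conditions.
; ResolveQTE restores time dilation, then either ragdolls the enemy and adds to the player's coin score, or opens the lose screen.
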(event OnComponentBeginOverlap(AttackRange)
  (params (OverlappedComponent :type Primitive%20Component%20Object%20Reference) (OtherActor :type Actor%20Object%20Reference) (OtherComp :type Primitive%20Component%20Object%20Reference) (OtherBodyIndex :type Integer) (bFromSweep :type Boolean) (SweepResult :type Hit%20Result%20Structure%20%28by%20ref%29))
  ;[0.15 0.15 0.15 0.5] Attack Range!
  (Utilities|Casting|CastToBP_CharacterMovement OtherActor) ; Same here
  (Variables|Default|SetbPlayerInAttackRange true))

(event OnComponentBeginOverlap(VisionDetection)
  (params (OverlappedComponent :type Primitive%20Component%20Object%20Reference) (OtherActor :type Actor%20Object%20Reference) (OtherComp :type Primitive%20Component%20Object%20Reference) (OtherBodyIndex :type Integer) (bFromSweep :type Boolean) (SweepResult :type Hit%20Result%20Structure%20%28by%20ref%29))
  ;[0.15 0.15 0.15 0.5] Vision Range!
  (bind _asbp_character_movement (Utilities|Casting|CastToBP_CharacterMovement OtherActor)) ; Makes only this character affect the\nCollision
  (Variables|Default|SetPlayerCharacter _asbp_character_movement)
  (Variables|Default|SetbSeesPlayer true))

(event EventBeginPlay
  ;[0.15 0.15 0.15 0.5] Sets variables and conditions needed for the enemy
  (Variables|Default|SetPatrolSpeed 0.4)
  (Variables|Default|SetbSeesPlayer false) ; Condition for transition from\nPatrol state to Stare state (StateTree)
  (Variables|Default|SetbPlayerInAttackRange false) ; Condition for transition from\nStare state to Attack (StateTree)
  (Variables|Default|SetQTEComplete false) ; Condition for if QTE is complete in\nAttack state (StateTree)
)

(event Collision|EventActorBeginOverlap
  (params (OtherActor :type Actor%20Object%20Reference)))

(event EventTick
  (params (DeltaSeconds :type Float%20%28single-precision%29))
  ;[0.15 0.15 0.15 0.5] Previous Blueprints, moved to STT statetree tasks
)

(fn ConstructionScript)

(fn ResolveQTE
  ;[0.15 0.15 0.15 0.5] What happens when the QTE is finished
  (Utilities|Time|SetGlobalTimeDilation 1.0)
  (if (Variables|Default|GetbSuccess)
    (Physics|SetSimulatePhysics (Variables|Default|GetEnemy) true) ; Makes Enemy ragdoll
    ;;[0.15 0.15 0.15 0.5] Adds to score when succeeded
    (Variables|/Game/Characters/BP_CharacterMovement.BP_CharacterMovement_C|SetCoinScore (Variables|Default|GetPlayerCharacter) (+ (Variables|/Game/Characters/BP_CharacterMovement.BP_CharacterMovement_C|GetCoinScore (Variables|Default|GetPlayerCharacter)) 10))
    (else
      (Game|OpenLevel(byObjectReference) "/Game/Levels/LoseScreen.LoseScreen"))))